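; Player character Blueprint that stores a gun reference at BeginPlay and handles the pause menu.
; The P key toggles game pause, adding or removing the pause menu widget and switching mouse cursor and input mode between UI-only and game-only.
; A level-name switch precedes the toggle but has only a default branch.
; Player HUD creation and its hookup to the building manager and gun component are present but never run.
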(event EventBeginPlay
  (Variables|Default|SetGun (Variables|Default|GetGun_BP)))

(event Collision|EventActorBeginOverlap
  (params (OtherActor :type Actor%20Object%20Reference)))

(event EventTick
  (params (DeltaSeconds :type Float%20%28single-precision%29)))

(event Input|KeyboardEvents|P
  (params (Key :type Key%20Structure))
  (bind _returnvalue (Game|GetPlayerController 0))
  (:Pressed
    (bind _returnvalue_2 (Game|GetCurrentLevelName true))
    (switch string _returnvalue_2
      (:Default
        (if (Game|IsGamePaused)
          (Game|SetGamePaused false)
          (Widget|RemovefromParent (stale _returnvalue_3))
          (Variables|/Script/Engine.PlayerController|SetbShowMouseCursor _returnvalue false)
          (Input|SetInputModeGameOnly _returnvalue false)
          (else
            (Game|SetGamePaused true)
            (bind _returnvalue_3 (UserInterface|CreateWidget "/Game/UI/PauseMenu_WBP.PauseMenu_WBP_C"))
            (UserInterface|Viewport|AddtoViewport _returnvalue_3 0)
            (Variables|/Script/Engine.PlayerController|SetbShowMouseCursor _returnvalue true)
            (Input|SetInputModeUIOnly _returnvalue 0 "DoNotLock" true)))))))

(fn ConstructionScript
  (|CallParentFunction))