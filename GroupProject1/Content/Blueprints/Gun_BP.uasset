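; Player gun for a building-demolition shooter, with five bullet types on number keys and an unlimited-feeling ammo count in the Tutorial level.
; Left click spawns the selected bullet at the camera, impulses its meshes forward, then updates the HUD count.
; At zero ammo, Tick reads BuildingManager's percent and, after a delay, shows the lose screen if short of the requirement.
; HUD lookup and manager registration are disconnected.
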(event EventBeginPlay
  (Variables|Default|SetBullet "/Game/Blueprints/BulletType1_BP.BulletType1_BP_C")
  (bind _returnvalue (Game|GetCurrentLevelName true))
  (if (Utilities|Enum|Equal(Enum) _returnvalue "Tutorial")
    (Variables|Default|SetBulletCount 10000)
    (Default|UpdateBullets (Variables|Default|GetPlayerHUD) self)))

(event EventTick
  (params (DeltaSeconds :type Float%20%28single-precision%29))
  (bind _returnvalue (Game|GetPlayerController 0))
  (if (== (Variables|Default|GetBulletCount) 0)
    (bind _returnvalue_2 (Actor|GetActorOfClass "/Game/Blueprints/BuildingManager_Blueprint.BuildingManager_Blueprint_C"))
    (Variables|Default|SetBuildingManager _returnvalue_2)
    (bind _percent (Default|GetPercent (Variables|Default|GetBuildingManager)))
    (Utilities|FlowControl|Delay 5.0)
    (if (not (and (>= _percent (Variables|/Game/Blueprints/BuildingManager_Blueprint.BuildingManager_Blueprint_C|GetRequiredPercent (Variables|Default|GetBuildingManager))) (== (Variables|Default|GetBulletCount) 0)))
      (bind _returnvalue_3 (UserInterface|CreateWidget "/Game/UI/EndScreen_WBP.EndScreen_WBP_C"))
      (UserInterface|Viewport|AddtoViewport _returnvalue_3 0)
      (Variables|/Script/Engine.PlayerController|SetbShowMouseCursor _returnvalue true)
      (Input|SetInputModeUIOnly _returnvalue 0 "DoNotLock" false)
      (Default|SetWinLoss _returnvalue_3 "You Lose!"))))

(event Input|MouseEvents|LeftMouseButton
  (params (Key :type Key%20Structure :default "None"))
  (bind _returnvalue (Game|GetPlayerController 0))
  (bind (_location _rotation) (Pawn|GetPlayerViewPoint _returnvalue))
  (:Pressed
    (if (> (Variables|Default|GetBulletCount) 0)
      (bind _returnvalue_2 (Game|SpawnActorfromClass (Variables|Default|GetBullet) (Math|Transform|MakeTransform _location _rotation "1.000000,1.000000,1.000000") "Undefined" 0 0))
      (for _array_element (Actor|GetComponentsByClass _returnvalue_2 "/Script/Engine.StaticMeshComponent")
        (Physics|AddImpulse _array_element (* (Math|Vector|GetForwardVector _rotation) 5e+05) "None" false))
      (Math|Integer|DecrementInt (Variables|Default|GetBulletCount)
        (:%20%20
          (Default|UpdateBullets (Variables|Default|GetPlayerHUD) self))))))

(event Input|KeyboardEvents|1
  (params (Key :type Key%20Structure :default "None"))
  (:Pressed
    (Variables|Default|SetBullet "/Game/Blueprints/BulletType1_BP.BulletType1_BP_C")))

(event Input|KeyboardEvents|2
  (params (Key :type Key%20Structure :default "None"))
  (:Pressed
    (Variables|Default|SetBullet "/Game/Blueprints/BulletType2_BP.BulletType2_BP_C")))

(event Input|KeyboardEvents|3
  (params (Key :type Key%20Structure :default "None"))
  (:Pressed
    (Variables|Default|SetBullet "/Game/Blueprints/BulletType3_BP.BulletType3_BP_C")))

(event Input|KeyboardEvents|4
  (params (Key :type Key%20Structure :default "None"))
  (:Pressed
    (Variables|Default|SetBullet "/Game/Blueprints/BulletType4_BP.BulletType4_BP_C")))

(event Input|KeyboardEvents|5
  (params (Key :type Key%20Structure :default "None"))
  (:Pressed
    (Variables|Default|SetBullet "/Game/Blueprints/BulletType5_BP.BulletType5_BP_C")))