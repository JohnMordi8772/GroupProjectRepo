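; Building manager that tracks how much of a brick building is destroyed and ends the level once a required percentage is reached.
; On BeginPlay it counts all Brick_Blueprint actors and creates the HUD; UpdateTotal decrements the remaining count.
; Tick polls the rounded destroyed fraction to refresh the HUD.
; At the threshold, a five-second Delay precedes the end screen, which shows the recomputed percentage with UI-only input.
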(event EventBeginPlay
  (bind _outactors (Actor|GetAllActorsOfClass "/Game/Blueprints/Brick_Blueprint.Brick_Blueprint_C"))
  (bind _output_get (Variables|Default|SetBricks _outactors))
  (bind _output_get_2 (Variables|Default|SetTotalBricks (Utilities|Array|Length _output_get)))
  (Variables|Default|SetCurrentBricks _output_get_2)
  (bind _returnvalue (UserInterface|CreateWidget "/Game/Blueprints/PlayerHUD.PlayerHUD_C"))
  (UserInterface|Viewport|AddtoViewport _returnvalue 0)
  (bind _output_get_3 (Variables|Default|SetHUD _returnvalue))
  (Variables|/Game/Blueprints/PlayerHUD.PlayerHUD_C|SetManager _output_get_3 self)
  (Default|UpdateText _output_get_3 0.0)
  (Rendering|Components|TextRender|SetText (Variables|/Game/Blueprints/PlayerHUD.PlayerHUD_C|GetRequiredDestruction (Variables|Default|GetHUD)) (Utilities|Text|FormatText (Class|KismetTextLibrary|AsPercentFloat (Variables|Default|GetRequiredPercent) "HalfToEven") (Utilities|Text|MakeLiteralText "%"))))

(event Collision|EventActorBeginOverlap
  (params (OtherActor :type Actor%20Object%20Reference)))

(event EventTick
  (params (DeltaSeconds :type Float%20%28single-precision%29))
  (bind _returnvalue (Game|GetPlayerController 0))
  (if (not (Variables|Default|GetEndWidetMade))
    (bind _percent (CallFunction|GetPercent))
    (Default|UpdateText (Variables|Default|GetHUD) _percent)
    (if (>= _percent (Variables|Default|GetRequiredPercent))
      (Utilities|FlowControl|Delay 5.0)
      (bind _returnvalue_2 (UserInterface|CreateWidget "/Game/UI/EndScreen_WBP.EndScreen_WBP_C"))
      (UserInterface|Viewport|AddtoViewport _returnvalue_2 0)
      (Variables|/Script/Engine.PlayerController|SetbShowMouseCursor _returnvalue true)
      (Input|SetInputModeUIOnly _returnvalue 0 "DoNotLock" false)
      (bind _percent_2 (CallFunction|GetPercent))
      (Default|UpdateEndText _returnvalue_2 _percent_2)
      (Variables|Default|SetEndWidetMade true))))

(fn ConstructionScript)

(fn UpdateTotal
  (Variables|Default|SetCurrentBricks (- (Variables|Default|GetCurrentBricks) 1)))

(fn GetPercent
  (return (/ (Math|Conversions|ToFloat(Integer) (Math|Float|Round (* (- 1.0 (/ (Math|Conversions|ToFloat(Integer) (Variables|Default|GetCurrentBricks)) (Math|Conversions|ToFloat(Integer) (Variables|Default|GetTotalBricks)))) 1e+02))) 1e+02)))