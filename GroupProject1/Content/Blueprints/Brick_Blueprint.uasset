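; Brick actor for a destructible building that loses durability from physics impacts and reports its destruction to a BuildingManager_Blueprint.
; On hit, it takes the faster linear speed of its own mesh and the other actor's static mesh.
; Speeds above Resistance are subtracted from Durability.
; At zero durability it disables collision, calls the manager's UpdateTotal and hides itself rather than being destroyed.
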(event OnComponentHit(StaticMeshComponent)
  (params (HitComponent :type Primitive%20Component%20Object%20Reference) (OtherActor :type Actor%20Object%20Reference) (OtherComp :type Primitive%20Component%20Object%20Reference) (NormalImpulse :type Vector :default "0, 0, 0") (Hit :type Hit%20Result%20Structure%20%28by%20ref%29))
  (if (> (Variables|Default|GetDurability) 0.0)
    (bind _returnvalue (Physics|GetPhysicsLinearVelocity (Actor|GetComponentbyClass OtherActor "/Script/Engine.StaticMeshComponent") "None"))
    (bind _returnvalue_2 (Physics|GetPhysicsLinearVelocity (Variables|Debug|GetStaticMeshComponent) "None"))
    (if (> (Math|Float|Max(Float) (Math|Vector|VectorLength _returnvalue_2) (Math|Vector|VectorLength _returnvalue)) (Variables|Default|GetResistance))
      (bind _output_get (Variables|Default|SetDurability (- (Variables|Default|GetDurability) (Math|Float|Max(Float) (Math|Vector|VectorLength _returnvalue_2) (Math|Vector|VectorLength _returnvalue)))))
      (if (<= _output_get 0.0)
        (Collision|SetActorEnableCollision false)
        (Default|UpdateTotal (Variables|Default|GetManager))
        (Rendering|SetActorHiddenInGame true)))))

(event EventBeginPlay
  (bind _returnvalue (Actor|GetActorOfClass "/Game/Blueprints/BuildingManager_Blueprint.BuildingManager_Blueprint_C"))
  (Variables|Default|SetManager _returnvalue))

(event Collision|EventActorBeginOverlap
  (params (OtherActor :type Actor%20Object%20Reference)))

(event EventTick
  (params (DeltaSeconds :type Float%20%28single-precision%29)))

(fn ConstructionScript)

(fn GetDurability
  (return (Variables|Default|GetDurability)))